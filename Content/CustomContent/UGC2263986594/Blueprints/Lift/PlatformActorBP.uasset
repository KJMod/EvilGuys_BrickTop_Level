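; PlatformActorBP is a moving platform from the Lift folder that travels back and forth continuously.
; On BeginPlay, the MovingPlatform component gets one of ten colour materials at random.
; Tick advances CurrentZPosition by Speed and delta time, flipping GoingUp at MaxRange and zero.
; Despite the Z naming, that value drives the component's relative Y, with X and Z zeroed, teleporting without sweep.
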(event `self.ReceiveBeginPlay`
  (`PrimitiveComponent.SetMaterial` (`self.MovingPlatform`) 0 (select `int` (`KismetMathLibrary.RandomIntegerInRange` 0 9) :`0` "/Game/CustomContent/UGC2263986594/Materials/M_Blue.M_Blue" :`1` "/Game/CustomContent/UGC2263986594/Materials/M_Red.M_Red" :`2` "/Game/CustomContent/UGC2263986594/Materials/M_Orange.M_Orange" :`3` "/Game/CustomContent/UGC2263986594/Materials/M_Yellow.M_Yellow" :`4` "/Game/CustomContent/UGC2263986594/Materials/M_Purple.M_Purple" :`5` "/Game/CustomContent/UGC2263986594/Materials/M_Green.M_Green" :`6` "/Game/CustomContent/UGC2263986594/Materials/M_DarkBlue.M_DarkBlue" :`7` "/Game/CustomContent/UGC2263986594/Materials/M_Cyan.M_Cyan" :`8` "/Game/CustomContent/UGC2263986594/Materials/M_Pink.M_Pink" :`9` "/Game/CustomContent/UGC2263986594/Materials/M_Salmon.M_Salmon" :!type "MaterialInterface Object Reference")))

(event `self.ReceiveTick`
  (params (DeltaSeconds :type "Float (single-precision)"))
  (bind _returnvalue (* (`self.Speed`) DeltaSeconds))
  (if (`self.bGoingUp`)
    (bind _output_get (set `self.CurrentZPosition` (+ (`self.CurrentZPosition`) _returnvalue)))
    (if (>= _output_get (`self.MaxRange`))
      (set `self.bGoingUp` false))
    (else
      (bind _output_get_2 (set `self.CurrentZPosition` (- (`self.CurrentZPosition`) _returnvalue)))
      (if (<= _output_get_2 0.0)
        (set `self.bGoingUp` true))))
  (`SceneComponent.K2_SetRelativeLocation` (`self.MovingPlatform`) (`KismetMathLibrary.MakeVector` 0.0 (`self.CurrentZPosition`)) false true))

(fn `UserConstructionScript`)