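; LargeCentralRotatorBP is a large central rotator prop whose spinner turns continuously.
; On BeginPlay, unless CustomColors is set, each Center and Spinner mesh gets its own random pick from six colored materials.
; Tick adds yaw to the main Spinner component, scaled by Speed and delta time for frame-rate independent rotation.
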(event `self.ReceiveBeginPlay`
  (bind _returnvalue (select `int` (`KismetMathLibrary.RandomIntegerInRange` 0 5) :`0` "/Game/CustomContent/UGC2263986594/Materials/M_Blue.M_Blue" :`1` "/Game/CustomContent/UGC2263986594/Materials/M_Red.M_Red" :`2` "/Game/CustomContent/UGC2263986594/Materials/M_Orange.M_Orange" :`3` "/Game/CustomContent/UGC2263986594/Materials/M_Yellow.M_Yellow" :`4` "/Game/CustomContent/UGC2263986594/Materials/M_Purple.M_Purple" :`5` "/Game/CustomContent/UGC2263986594/Materials/M_Green.M_Green" :!type "MaterialInterface Object Reference"))
  (if (not (`self.CustomColors`))
    (`PrimitiveComponent.SetMaterial` (`self.Center`) 0 _returnvalue)
    (`PrimitiveComponent.SetMaterial` (`self.Center1`) 0 _returnvalue)
    (`PrimitiveComponent.SetMaterial` (`self.Center2`) 0 _returnvalue)
    (`PrimitiveComponent.SetMaterial` (`self.Center3`) 0 _returnvalue)
    (`PrimitiveComponent.SetMaterial` (`self.Spinner`) 0 _returnvalue)
    (`PrimitiveComponent.SetMaterial` (`self.Spinner1`) 0 _returnvalue)
    (`PrimitiveComponent.SetMaterial` (`self.Spinner2`) 0 _returnvalue)))

(event `self.ReceiveTick`
  (params (DeltaSeconds :type "Float (single-precision)"))
  (`SceneComponent.K2_AddRelativeRotation` (`self.Spinner`) (`KismetMathLibrary.MakeRotator` 0.0 0.0 (* DeltaSeconds (`self.Speed`))) false false))

(fn `UserConstructionScript`)