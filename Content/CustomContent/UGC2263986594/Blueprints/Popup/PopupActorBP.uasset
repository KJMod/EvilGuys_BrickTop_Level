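; PopupActorBP is an actor whose Popup component repeatedly moves along its Z axis at random intervals.
; BeginPlay assigns random colors from a light or dark palette, chosen by DarkScheme, to most Base material slots and to the Popup.
; On authority, a Delay in Tick acts as a repeating timer, re-rolling between MinDelay and MaxDelay before calling FireEvent.
; FireEvent restarts PopupTimeline, which drives the Popup's relative height.
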(event `self.ReceiveBeginPlay`
  (bind _returnvalue (`KismetMathLibrary.RandomIntegerInRange` 0 5))
  (bind _returnvalue_2 (select `bool` (`self.DarkScheme`) :`false` (select `int` _returnvalue :`0` "/Game/CustomContent/UGC2263986594/Materials/M_Blue.M_Blue" :`1` "/Game/CustomContent/UGC2263986594/Materials/M_Red.M_Red" :`2` "/Game/CustomContent/UGC2263986594/Materials/M_Orange.M_Orange" :`3` "/Game/CustomContent/UGC2263986594/Materials/M_Yellow.M_Yellow" :`4` "/Game/CustomContent/UGC2263986594/Materials/M_Purple.M_Purple" :`5` "/Game/CustomContent/UGC2263986594/Materials/M_Green.M_Green" :!type "MaterialInterface Object Reference") :`true` (select `int` _returnvalue :`0` "/Game/CustomContent/UGC2263986594/Materials/Dark/M_Blue_Dark.M_Blue_Dark" :`1` "/Game/CustomContent/UGC2263986594/Materials/Dark/M_Red_Dark.M_Red_Dark" :`2` "/Game/CustomContent/UGC2263986594/Materials/Dark/M_Orange_Dark.M_Orange_Dark" :`3` "/Game/CustomContent/UGC2263986594/Materials/Dark/M_Yellow_Dark.M_Yellow_Dark" :`4` "/Game/CustomContent/UGC2263986594/Materials/Dark/M_Purple_Dark.M_Purple_Dark" :`5` "/Game/CustomContent/UGC2263986594/Materials/Dark/M_Green_Dark.M_Green_Dark" :!type "MaterialInterface Object Reference")))
  (`PrimitiveComponent.SetMaterial` (`self.Base`) 0 _returnvalue_2)
  (`PrimitiveComponent.SetMaterial` (`self.Base`) 1 _returnvalue_2)
  (`PrimitiveComponent.SetMaterial` (`self.Base`) 2 _returnvalue_2)
  (`PrimitiveComponent.SetMaterial` (`self.Base`) 3 _returnvalue_2)
  (`PrimitiveComponent.SetMaterial` (`self.Base`) 5 _returnvalue_2)
  (`PrimitiveComponent.SetMaterial` (`self.Popup`) 0 _returnvalue_2)
  (set `self.RandomDelay` (`KismetMathLibrary.RandomFloatInRange` 0.0 1.0)))

(event `self.ReceiveTick`
  (params (DeltaSeconds :type "Float (single-precision)"))
  (`/Engine/EditorBlueprintResources/ActorMacros.Switch Has Authority`
    (:`Authority`
      (`KismetSystemLibrary.Delay` (`self.RandomDelay`))
      (set `self.RandomDelay` (`KismetMathLibrary.RandomFloatInRange` (`self.MinDelay`) (`self.MaxDelay`)))
      (`self.FireEvent`))))

(event `FireEvent`
  (bind (_direction _newtrack_0) (`Timeline|PopupTimeline` :!via `PlayFromStart`)
    (:`Update`
      (`SceneComponent.K2_SetRelativeLocation` (`self.Popup`) (`KismetMathLibrary.MakeVector` 0.0 0.0 _newtrack_0) false true))))

(fn `UserConstructionScript`)