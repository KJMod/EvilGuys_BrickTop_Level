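; Pusher obstacle actor: a piston that pops out and retracts at random intervals with a cartoon sound.
; On the authority, Tick uses a Delay as a repeating random timer that calls FireEvent with a random pause.
; FireEvent plays one timeline out and, after the pause, another back, teleporting Popup along Z with travel adjusted by LengthMultiplier.
; BeginPlay scales Popup by that multiplier and randomizes mesh colors unless CustomColors is set.
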(event `self.ReceiveBeginPlay`
  (bind _returnvalue (select `int` (`KismetMathLibrary.RandomIntegerInRange` 0 5) :`0` "/Game/CustomContent/UGC2263986594/Materials/M_Blue.M_Blue" :`1` "/Game/CustomContent/UGC2263986594/Materials/M_Red.M_Red" :`2` "/Game/CustomContent/UGC2263986594/Materials/M_Orange.M_Orange" :`3` "/Game/CustomContent/UGC2263986594/Materials/M_Yellow.M_Yellow" :`4` "/Game/CustomContent/UGC2263986594/Materials/M_Purple.M_Purple" :`5` "/Game/CustomContent/UGC2263986594/Materials/M_Green.M_Green" :!type "MaterialInterface Object Reference"))
  (`SceneComponent.SetRelativeScale3D` (`self.Popup`) (`KismetMathLibrary.MakeVector` (`self.LengthMultiplier`) 2.0 2.0))
  (if (not (`self.CustomColors`))
    (`PrimitiveComponent.SetMaterial` (`self.Base`) 0 _returnvalue)
    (`PrimitiveComponent.SetMaterial` (`self.Popup`) 0 _returnvalue)
    (`PrimitiveComponent.SetMaterial` (`self.StaticMesh`) 0 _returnvalue)
    (`PrimitiveComponent.SetMaterial` (`self.StaticMesh2`) 0 _returnvalue)
    (`PrimitiveComponent.SetMaterial` (`self.StaticMesh3`) 0 _returnvalue)
    (`PrimitiveComponent.SetMaterial` (`self.StaticMesh4`) 0 _returnvalue)
    (`PrimitiveComponent.SetMaterial` (`self.StaticMesh5`) 0 _returnvalue)
    (`PrimitiveComponent.SetMaterial` (`self.StaticMesh6`) 0 _returnvalue)
    (`PrimitiveComponent.SetMaterial` (`self.StaticMesh7`) 0 _returnvalue))
  (set `self.RandomDelay` (`KismetMathLibrary.RandomFloatInRange` 0.0 1.0)))

(event `self.ReceiveTick`
  (params (DeltaSeconds :type "Float (single-precision)"))
  (`/Engine/EditorBlueprintResources/ActorMacros.Switch Has Authority`
    (:`Authority`
      (`KismetSystemLibrary.Delay` (`self.RandomDelay`))
      (set `self.RandomDelay` (`KismetMathLibrary.RandomFloatInRange` (`self.MinDelay`) (`self.MaxDelay`)))
      (`self.FireEvent` (`KismetMathLibrary.RandomFloatInRange` (`self.PauseMin`) (`self.PauseMax`))))))

(event `FireEvent`
  (params (OutDelay :type "Float (double-precision)"))
  (`AudioComponent.Play` (`self.CartoonPistonSoundCue`) 0.0)
  (bind (_direction _newtrack_0) (`Timeline|PopupTimeline` :`NewTime` 0.0 :!via `PlayFromStart`)
    (:`Update`
      (`SceneComponent.K2_SetRelativeLocation` (`self.Popup`) (`KismetMathLibrary.MakeVector` 0.0 0.0 (* (- _newtrack_0 (/ 50.0 (`self.LengthMultiplier`))) (`self.LengthMultiplier`))) false true))
    (:`Finished`
      (`KismetSystemLibrary.Delay` OutDelay)
      (bind (_direction_2 _newtrack_0_2) (`Timeline|Timeline_0` :!via `PlayFromStart`)
        (:`Update`
          (`SceneComponent.K2_SetRelativeLocation` (`self.Popup`) (`KismetMathLibrary.MakeVector` 0.0 0.0 (* (- _newtrack_0_2 (/ 50.0 (`self.LengthMultiplier`))) (`self.LengthMultiplier`))) false true))))))

(fn `UserConstructionScript`)