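; Respawn trigger actor that teleports any Character overlapping it to a random destination in the level.
; On overlap it gathers all actors carrying the TaggedActorLabel tag and uses random picks from them for the teleport location and rotation.
; It then stops the character's movement immediately and zeroes its velocity, so no momentum carries through the teleport.
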(event `self.ReceiveActorBeginOverlap`
  (params (OtherActor :type "Actor Object Reference"))
  (bind _ascharacter (cast `Character` OtherActor))
  (bind _outactors (`GameplayStatics.GetAllActorsWithTag` (`self.TaggedActorLabel`)))
  (bind _output (`|GetArrayItem` _outactors (`KismetMathLibrary.RandomInteger` (`KismetArrayLibrary.Array_Length` _outactors))))
  (`self.K2_TeleportTo` _ascharacter (`self.K2_GetActorLocation` _output) (`self.K2_GetActorRotation` _output))
  (`MovementComponent.StopMovementImmediately` (`Pawn.GetMovementComponent` _ascharacter))
  (set `MovementComponent.Velocity` (0.0 0.0 0.0) (`Character.CharacterMovement` _ascharacter)))

(fn `UserConstructionScript`)